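; Key actor for the train station that shows close or far prompt widgets until it is grabbed.
; SetPrompt switches on PromptType to show the close widget, the far widget or neither, and does nothing once Grabbed is true.
; Tick hides both widgets every frame while the key is grabbed.
; Grabbed and PromptType are only read in these graphs, never set.
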(event `self.ReceiveTick`
  (params (DeltaSeconds :type "Float (single-precision)"))
  (if (`self.Grabbed`)
    (`SceneComponent.SetVisibility` (`self.CloseWidget`) false false)
    (`SceneComponent.SetVisibility` (`self.Far Widget`) false false)))

(event `self.SetPrompt`
  (if (not (`self.Grabbed`))
    (switch `int` (`self.PromptType`)
      (:`Default`
        (`SceneComponent.SetVisibility` (`self.CloseWidget`) false false)
        (`SceneComponent.SetVisibility` (`self.Far Widget`) false false))
      (:`0`
        (`SceneComponent.SetVisibility` (`self.CloseWidget`) false false)
        (`SceneComponent.SetVisibility` (`self.Far Widget`) false false))
      (:`1`
        (`SceneComponent.SetVisibility` (`self.CloseWidget`) true false)
        (`SceneComponent.SetVisibility` (`self.Far Widget`) false false))
      (:`2`
        (`SceneComponent.SetVisibility` (`self.CloseWidget`) false false)
        (`SceneComponent.SetVisibility` (`self.Far Widget`) true false)))))

(fn `UserConstructionScript`)