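; BP_ManualLight_Lamp_Double is a double lamp object whose secondary lights and visuals follow the state of its main SpotLight.
; BeginPlay hides both sets of rect light, plane and W components, plus SpotLight2.
; Every Tick then polls SpotLight visibility, copies it to those components, and swaps StaticMesh1's material between lit and unlit.
; The graph never toggles SpotLight itself, only mirrors it.
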(event `self.ReceiveBeginPlay`
  (`parent.ReceiveBeginPlay`)
  (`|ExecutionSequence`
    (:`then_0`
      (`SceneComponent.SetVisibility` (`self.w`) false false)
      (`SceneComponent.SetVisibility` (`self.RectLight`) false false)
      (`SceneComponent.SetVisibility` (`self.Plane`) false false))
    (:`then_1`
      (`SceneComponent.SetVisibility` (`self.w1`) false false)
      (`SceneComponent.SetVisibility` (`self.RectLight1`) false false)
      (`SceneComponent.SetVisibility` (`self.Plane1`) false false)
      (`SceneComponent.SetVisibility` (`self.SpotLight2`) false false))))

(event `self.ReceiveTick`
  (params (DeltaSeconds :type "Float (single-precision)"))
  (bind _returnvalue (`SceneComponent.IsVisible` (`self.SpotLight`)))
  (`parent.ReceiveTick` DeltaSeconds)
  (`|ExecutionSequence`
    (:`then_0`
      (`SceneComponent.SetVisibility` (`self.w`) _returnvalue false)
      (`SceneComponent.SetVisibility` (`self.RectLight`) _returnvalue false)
      (`SceneComponent.SetVisibility` (`self.Plane`) _returnvalue false)
      (`SceneComponent.SetVisibility` (`self.w1`) _returnvalue false)
      (`SceneComponent.SetVisibility` (`self.RectLight1`) _returnvalue false)
      (`SceneComponent.SetVisibility` (`self.Plane1`) _returnvalue false)
      (`SceneComponent.SetVisibility` (`self.SpotLight2`) _returnvalue false))
    (:`then_1`
      (if _returnvalue
        (`PrimitiveComponent.SetMaterial` (`self.StaticMesh1`) (`self.TexNum`) "/Game/Materials/Light_Mat.Light_Mat")
        (else
          (`PrimitiveComponent.SetMaterial` (`self.StaticMesh1`) (`self.TexNum`) "/Game/Materials/Light_Off_Mat.Light_Off_Mat"))))))

(fn `UserConstructionScript`
  (`parent.UserConstructionScript`))