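; BP_ElevatorClicker is an elevator button object with a cylinder mesh and a point light that show whether it is active.
; Every Tick it checks the IsOn and HasPower flags, lighting the point light and applying the on material only when both are true, otherwise using the off material and hiding the light.
; The Blueprint only displays this state and does not set either flag itself.
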(event `self.ReceiveTick`
  (params (DeltaSeconds :type "Float (single-precision)"))
  (if (and (`self.IsOn`) (`self.HasPower`))
    (`PrimitiveComponent.SetMaterial` (`self.Cylinder`) 0 (`self.OnMatt`))
    (`SceneComponent.SetVisibility` (`self.PointLight`) true false)
    (else
      (`PrimitiveComponent.SetMaterial` (`self.Cylinder`) 0 (`self.OffMat`))
      (`SceneComponent.SetVisibility` (`self.PointLight`) false false))))

(fn `UserConstructionScript`)