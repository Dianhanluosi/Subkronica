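; BP_ManualLight_Sqaure1 is a light actor that extends a parent Blueprint, adding visibility sync between its components.
; On BeginPlay it runs the parent logic, then hides the W component and RectLight.
; Every Tick, after the parent update, it copies SpotLight's visibility to both, so they follow the spot light by polling rather than events.
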(event `self.ReceiveBeginPlay`
  (`parent.ReceiveBeginPlay`)
  (`SceneComponent.SetVisibility` (`self.w`) false false)
  (`SceneComponent.SetVisibility` (`self.RectLight`) false false))

(event `self.ReceiveTick`
  (params (DeltaSeconds :type "Float (single-precision)"))
  (bind _returnvalue (`SceneComponent.IsVisible` (`self.SpotLight`)))
  (`parent.ReceiveTick` DeltaSeconds)
  (`SceneComponent.SetVisibility` (`self.w`) _returnvalue false)
  (`SceneComponent.SetVisibility` (`self.RectLight`) _returnvalue false))

(fn `UserConstructionScript`
  (`parent.UserConstructionScript`))