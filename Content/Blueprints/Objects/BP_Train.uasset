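; BP_Train is a train object whose lights switch on or off to match its HasPower flag.
; BeginPlay gathers the light fixture meshes and point lights into two arrays.
; Every Tick, it polls HasPower, swaps each mesh's first material between lit and unlit versions, and sets point light visibility to match.
; The file never sets HasPower, and the lighting is reapplied each frame even without a change.
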(event `self.ReceiveBeginPlay`
  (set `self.LightMesh` (`|MakeArray` (`self.StaticMesh2`) (`self.StaticMesh3`) (`self.StaticMesh4`) (`self.StaticMesh5`) (`self.StaticMesh7`) (`self.StaticMesh6`) (`self.StaticMesh8`) (`self.StaticMesh9`) (`self.StaticMesh10`) (`self.StaticMesh1`) (`self.StaticMesh11`) (`self.StaticMesh`)))
  (set `self.PointLights` (`|MakeArray` (`self.PointLight`) (`self.PointLight1`) (`self.PointLight2`) (`self.PointLight3`))))

(event `self.ReceiveTick`
  (params (DeltaSeconds :type "Float (single-precision)"))
  (if (`self.HasPower`)
    (`|ExecutionSequence`
      (:`then_0`
        (for _array_element (`self.LightMesh`)
          (`PrimitiveComponent.SetMaterial` _array_element 0 "/Game/Materials/Light_Mat.Light_Mat")))
      (:`then_1`
        (for _array_element_2 (`self.PointLights`)
          (`SceneComponent.SetVisibility` _array_element_2 true false))))
    (else
      (`|ExecutionSequence`
        (:`then_0`
          (for _array_element_3 (`self.LightMesh`)
            (`PrimitiveComponent.SetMaterial` _array_element_3 0 "/Game/Materials/Light_Off_Mat.Light_Off_Mat")))
        (:`then_1`
          (for _array_element_4 (`self.PointLights`)
            (`SceneComponent.SetVisibility` _array_element_4 false false)))))))

(fn `UserConstructionScript`)