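; BP_AutoLight is a light fixture that switches on only while it has power and is alive.
; When SoundSensitive is set, it starts not alive, and Tick sets IsAlive from the player's distance and height difference, with no actual sound detection.
; Tick then reapplies the lit or unlit material on the static mesh and toggles the spotlight's visibility every frame.
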(event `self.ReceiveBeginPlay`
  (`PrimitiveComponent.SetMaterial` (`self.StaticMesh`) (`self.TexNum`) "/Game/Materials/Light_Off_Mat.Light_Off_Mat")
  (`SceneComponent.SetVisibility` (`self.SpotLight`) false false)
  (if (`self.SoundSensitive`)
    (set `self.IsAlive` false)))

(event `self.ReceiveTick`
  (params (DeltaSeconds :type "Float (single-precision)"))
  (bind _returnvalue (`GameplayStatics.GetPlayerCharacter` 0))
  (bind _texnum (`self.TexNum`))
  (`|ExecutionSequence`
    (:`then_0`
      (if (`self.SoundSensitive`)
        (if (and (<= (`self.GetDistanceTo` _returnvalue self) (`self.AliveDistance`)) (<= (`KismetMathLibrary.Abs` (- (.z (.location (`self.GetTransform` _returnvalue))) (.z (.location (`self.GetTransform` self))))) 2500.0))
          (set `self.IsAlive` true)
          (else
            (set `self.IsAlive` false)))))
    (:`then_1`
      (if (and (`self.HasPower`) (`self.IsAlive`))
        (`PrimitiveComponent.SetMaterial` (`self.StaticMesh`) _texnum "/Game/Materials/Light_Mat.Light_Mat")
        (`SceneComponent.SetVisibility` (`self.SpotLight`) true false)
        (else
          (`PrimitiveComponent.SetMaterial` (`self.StaticMesh`) _texnum "/Game/Materials/Light_Off_Mat.Light_Off_Mat")
          (`SceneComponent.SetVisibility` (`self.SpotLight`) false false))))))

(fn `UserConstructionScript`)