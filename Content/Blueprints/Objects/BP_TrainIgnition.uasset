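; Train ignition object that offers an interaction prompt and has a toggleable indicator light.
; Pressed activates the Ig component, which starts deactivated on BeginPlay, and prints a debug string.
; A separate Ignition event flips the Cylinder between lit and unlit materials and toggles the PointLight's visibility.
; SetPrompt switches on PromptType to show the close widget, the far widget or neither.
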(event `self.ReceiveBeginPlay`
  (`ActorComponent.Deactivate` (`self.Ig`)))

(event `self.Ignition`
  (bind _pointlight (`self.PointLight`))
  (`|ExecutionSequence`
    (:`then_0`
      (`|ExecutionSequence`
        (:`then_0`
          (if (== (`PrimitiveComponent.GetMaterial` (`self.Cylinder`) 0) "/Game/Materials/Light_Off_Mat.Light_Off_Mat")
            (`PrimitiveComponent.SetMaterial` (`self.Cylinder`) 0 "/Game/Materials/Light_Mat.Light_Mat")
            (else
              (`PrimitiveComponent.SetMaterial` (`self.Cylinder`) 0 "/Game/Materials/Light_Off_Mat.Light_Off_Mat"))))
        (:`then_1`
          (`SceneComponent.SetVisibility` _pointlight (not (`SceneComponent.bVisible` _pointlight)) false))))))

(event `self.Pressed`
  (`|ExecutionSequence`
    (:`then_0`
      (`ActorComponent.Activate` (`self.Ig`) false))
    (:`then_1`
      (`KismetSystemLibrary.PrintString` "Hello"))))

(event `self.SetPrompt`
  (switch `int` (`self.PromptType`)
    (:`Default`
      (`SceneComponent.SetVisibility` (`self.CloseWidget`) false false)
      (`SceneComponent.SetVisibility` (`self.Far Widget`) false false))
    (:`0`
      (`SceneComponent.SetVisibility` (`self.CloseWidget`) false false)
      (`SceneComponent.SetVisibility` (`self.Far Widget`) false false))
    (:`1`
      (`SceneComponent.SetVisibility` (`self.CloseWidget`) true false)
      (`SceneComponent.SetVisibility` (`self.Far Widget`) false false))
    (:`2`
      (`SceneComponent.SetVisibility` (`self.CloseWidget`) false false)
      (`SceneComponent.SetVisibility` (`self.Far Widget`) true false))))

(fn `UserConstructionScript`)