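; BP_Elevator is an elevator actor whose running sound and light follow its movement and power state.
; Every Tick it activates the SQElevatorRunning component while IsMoving and HasPower are both true, and deactivates it otherwise.
; The same Tick swaps the Light mesh between on and off materials and toggles the RectLight's visibility based on HasPower.
; The graph contains no movement logic and only reads those two flags.
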(event `self.ReceiveBeginPlay`)

(event `self.ReceiveTick`
  (params (DeltaSeconds :type "Float (single-precision)"))
  (bind _haspower (`self.HasPower`))
  (bind _sq_elevatorrunning (`self.SQ_ElevatorRunning`))
  (`|ExecutionSequence`
    (:`then_0`
      (if (and (`self.bIsMoving`) _haspower)
        (`ActorComponent.Activate` _sq_elevatorrunning false)
        (else
          (`ActorComponent.Deactivate` _sq_elevatorrunning))))
    (:`then_1`
      (if _haspower
        (`PrimitiveComponent.SetMaterial` (`self.Light`) 0 (`self.OnMat`))
        (`SceneComponent.SetVisibility` (`self.RectLight`) true false)
        (else
          (`PrimitiveComponent.SetMaterial` (`self.Light`) 0 (`self.OffMat`))
          (`SceneComponent.SetVisibility` (`self.RectLight`) false false))))))

(fn `UserConstructionScript`)