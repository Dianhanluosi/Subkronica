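; Powerplant spinner object that drives its lights, mesh material and humming sound from its on and spinning states.
; Tick toggles four rect lights and swaps on/off materials with IsSpinning, then ramps hum volume toward full or silent with IsOn.
; The fade time is derived from remaining rotation speed over acceleration, so the hum follows spin-up and spin-down.
; CallingEndingManager forwards to PowerSwitchCick's CallingAction.
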(event `self.ReceiveBeginPlay`
  (`PrimitiveComponent.SetMaterial` (`self.SpinnerMesh`) 0 (`self.OffMat`))
  (set `self.Volume` (`AudioComponent.VolumeMultiplier` (`self.SQ_SpinnerHumming`))))

(event `self.ReceiveTick`
  (params (DeltaSeconds :type "Float (single-precision)"))
  (bind _isspinning (`self.IsSpinning`))
  (bind _volume (`self.Volume`))
  (bind _volume_2 (`self.Volume`))
  (`|ExecutionSequence`
    (:`then_0`
      (for _array_element (`|MakeArray` (`self.RectLight1`) (`self.RectLight2`) (`self.RectLight4`) (`self.RectLight`))
        (`SceneComponent.SetVisibility` _array_element _isspinning false)
        (if _isspinning
          (`PrimitiveComponent.SetMaterial` (`self.SpinnerMesh`) 0 (`self.OnMat`))
          (else
            (`PrimitiveComponent.SetMaterial` (`self.SpinnerMesh`) 0 (`self.OffMat`))))))
    (:`then_1`
      (if (`self.IsOn`)
        (bind _output_get (set `self.VolumeSpeed` (/ (- 1.0 (`AudioComponent.VolumeMultiplier` (`self.SQ_SpinnerHumming`))) (`self.VolumeTime`))))
        (set `self.Volume` (+ (* _output_get DeltaSeconds) (`self.Volume`)))
        (else
          (bind _output_get_2 (set `self.VolumeSpeed` (/ (- (`AudioComponent.VolumeMultiplier` (`self.SQ_SpinnerHumming`)) 0.0) (`self.VolumeTime`))))
          (set `self.Volume` (- (`self.Volume`) (* _output_get_2 DeltaSeconds))))))
    (:`then_2`
      (if (`self.IsOn`)
        (`/Engine/EditorBlueprintResources/StandardMacros.CompareFloat` _volume_2 1.0
          (:`>`
            (`AudioComponent.SetVolumeMultiplier` (`self.SQ_SpinnerHumming`) 1.0))
          (:`<`
            (`AudioComponent.SetVolumeMultiplier` (`self.SQ_SpinnerHumming`) _volume_2)))
        (else
          (`/Engine/EditorBlueprintResources/StandardMacros.CompareFloat` _volume
            (:`>`
              (`AudioComponent.SetVolumeMultiplier` (`self.SQ_SpinnerHumming`) _volume))
            (:`<`
              (`AudioComponent.SetVolumeMultiplier` (`self.SQ_SpinnerHumming`) 0.0))))))
    (:`then_3`
      (if (`self.IsOn`)
        (set `self.VolumeTime` (/ (- (`self.TerminalRotationSpeed`) (`self.RotationSpeed`)) (`self.RotationAcceleration`)))
        (else
          (set `self.VolumeTime` (/ (- (`self.RotationSpeed`) 0.0) (`self.RotationAcceleration`))))))))

(event `self.CallingEndingManager`
  (`PowerSwitchClick.CallingAction` (`self.PowerSwitchCick`)))

(fn `UserConstructionScript`)