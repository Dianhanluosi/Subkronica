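; BP_WaterplantWheel is a waterplant wheel actor that handles winding and water audio plus interaction prompt widgets.
; The STO event plays the winding sound unless it is already playing.
; Tick polls SwitchedOn, activating the water sound after a one-second delay or deactivating it when off.
; SetPrompt uses PromptType to show the close widget, the far widget, or neither.
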(event `self.ReceiveBeginPlay`
  (`AudioComponent.Stop` (`self.SQ_Winding`)))

(event `self.ReceiveTick`
  (params (DeltaSeconds :type "Float (single-precision)"))
  (bind _sq_watersound (`self.SQ_WaterSound`))
  (if (`self.SwitchedOn`)
    (`KismetSystemLibrary.Delay` 1.0)
    (`ActorComponent.Activate` _sq_watersound false)
    (else
      (`ActorComponent.Deactivate` _sq_watersound))))

(event `self.STO`
  (bind _sq_winding (`self.SQ_Winding`))
  (if (not (`AudioComponent.IsPlaying` _sq_winding))
    (`AudioComponent.Play` _sq_winding 0.0)))

(event `self.SetPrompt`
  (switch `int` (`self.PromptType`)
    (:`Default`
      (`SceneComponent.SetVisibility` (`self.CloseWidget`) false false)
      (`SceneComponent.SetVisibility` (`self.Far Widget`) false false))
    (:`0`
      (`SceneComponent.SetVisibility` (`self.CloseWidget`) false false)
      (`SceneComponent.SetVisibility` (`self.Far Widget`) false false))
    (:`1`
      (`SceneComponent.SetVisibility` (`self.CloseWidget`) true false)
      (`SceneComponent.SetVisibility` (`self.Far Widget`) false false))
    (:`2`
      (`SceneComponent.SetVisibility` (`self.CloseWidget`) false false)
      (`SceneComponent.SetVisibility` (`self.Far Widget`) true false))))

(fn `UserConstructionScript`)