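; BP_FallEnding is a trigger actor that plays the fall ending when the player character overlaps its Ending_Collider.
; It fades the camera out over several seconds, then shows the WBP_Ending_BlackOut widget and reports the ending number to the first BP_EndingManager found in the level.
; After a further delay it opens the TownStart level.
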(event `self.Ending_Collider.OnComponentBeginOverlap`
  (params (OverlappedComponent :type "PrimitiveComponent Object Reference") (OtherActor :type "Actor Object Reference") (OtherComp :type "PrimitiveComponent Object Reference") (OtherBodyIndex :type Integer) (bFromSweep :type Boolean) (SweepResult :type "HitResult Structure (by ref)"))
  (cast `/Game/Blueprints/Pawns/BP_PlayerCharacter` OtherActor)
  (`|ExecutionSequence`
    (:`then_0`
      (`PlayerCameraManager.StartCameraFade` :`self` (`GameplayStatics.GetPlayerCameraManager` 0) :`ToAlpha` 1.0 :`Duration` 5.0))
    (:`then_1`
      (`KismetSystemLibrary.Delay` 5.0)
      (bind _returnvalue (`|CreateWidget` "/Game/UI/WBP_Ending_BlackOut.WBP_Ending_BlackOut_C"))
      (`UserWidget.AddToViewport` _returnvalue 0)
      (bind _outactors (`GameplayStatics.GetAllActorsOfClass` "/Game/Blueprints/GameMode/BP_EndingManager.BP_EndingManager_C"))
      (`EndingManager.ReceiveEndingNumber` (`|GetArrayItem` _outactors) 5)
      (`KismetSystemLibrary.Delay` 10.0)
      (`GameplayStatics.OpenLevel` "TownStart"))))

(fn `UserConstructionScript`)